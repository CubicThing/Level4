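; BP_Hori_Platform is an actor for a horizontally moving platform that shuttles between two points.
; When MBeginMove is set, BeginPlay starts a timeline that lerps the mesh's relative location from zero toward an X destination, without sweeping.
; Each time the timeline finishes, it flips the MMoveRight flag, initialized in the Construction Script, to choose between playing and reversing, intended as a continuous back-and-forth loop.
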(event `self.ReceiveBeginPlay`
  ;[1 1 1] Default call
  (if (`self.M BeginMove`)
    (`self.MoveRight`)))

(event `MoveRight`
  ;[1 1 1] Horizontal Platform animation
  (bind (_direction _x_force) (`Timeline|PlatformAnimation` :`NewTime` 10.0 :!label _label)
    (:`Update`
      (`SceneComponent.K2_SetRelativeLocation` (`self.PlatformMesh`) (`KismetMathLibrary.VLerp` (0.0 0.0 0.0) (`KismetMathLibrary.MakeVector` (`self.m_XDestination`)) _x_force) false false))
    (:`Finished`
      ;;[1 1 1] Resetting the direciton
      (bind _output_get (set `self.M MoveRight` (not (`self.M MoveRight`))))
      (if _output_get
        (`self.MoveLeft`)
        (else
          (`self.MoveRight`))))))

(event `MoveLeft`
  ;[1 1 1] Horizontal Platform animation
  (goto _label :!via `Reverse`))

(fn `UserConstructionScript`
  (set `self.M MoveRight` true))